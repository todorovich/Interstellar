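; RandomStar is a Blueprint that gives a star randomized properties.
; Its construction script rolls integer sector coordinates in a cube around the origin, a color temperature in Kelvin and a size in solar radii, so values re-roll whenever construction reruns.
; An unconnected spherical-coordinate calculation for position remains in the graph, and the event graph holds only disabled default events.
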(fn `UserConstructionScript`
  (set `self.SectorCoordinates` (make `IntVector` (- (`KismetMathLibrary.RandomInteger` 5000) 2500) (- (`KismetMathLibrary.RandomInteger` 5000) 2500) (- (`KismetMathLibrary.RandomInteger` 5000) 2500)))
  (set `self.ColorTemperatureKelvin` (+ (`KismetMathLibrary.RandomInteger` 5000) 1000))
  (set `self.SizeSolarRadii` (* (`KismetMathLibrary.RandomFloat`) 100000.0)))